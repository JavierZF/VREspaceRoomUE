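; Photon Cloud networking Blueprint that connects VR players to a shared four-player room and spawns their pawns.
; On initialization it connects under a random GUID name, while a short timer caches player starts from the local BP_VR_Controller.
; Once connected it joins or creates "VR-ROOM".
; Each join has the controller create a local or remote pawn at the start indexed by player number.
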(event Custom|On%20Fake%20Start
  ;[1 1 1] Save all player starts in the array
  (bind _asbp_vr_controller (Utilities|Casting|CastToBP_VR_Controller (Class|PhotonCloudAPIBPLibrary|GetFirstLocalPlayerController self)))
  (Variables|Config|SetPlayer%20Starts (Default|GetAllStarts _asbp_vr_controller)))

(event Custom|On%20Connect
  ;[1 1 1] Connect
  ;[1 1 1] Join a room
  (Class|PhotonCloudObject|JoinorCreateRoom "VR-ROOM" 4 0))

(event Custom|On%20Player%20Joined
  (params (PlayerNumber :type Integer) (PlayerName :type String) (IsLocalPlayer :type Boolean))
  (bind _returnvalue (- PlayerNumber 1))
  (bind _player_starts (Variables|Config|GetPlayer%20Starts))
  (bind _output (Utilities|Array|Get(acopy) _player_starts _returnvalue))
  (bind _returnvalue_2 (Transformation|GetActorTransform _output))
  ;[1 1 1] Join a room
  (Development|PrintString self (Utilities|String|Append PlayerName " joined : #" (Utilities|String|ToString(Integer) PlayerNumber)))
  (bind _asbp_vr_controller (Utilities|Casting|CastToBP_VR_Controller (Class|PhotonCloudAPIBPLibrary|GetFirstLocalPlayerController self))
    (:then
      (Default|CreatePawn _asbp_vr_controller (Math|Transform|MakeTransform (.location _returnvalue_2) (.rotation _returnvalue_2)) IsLocalPlayer))
    (:CastFailed
      (Development|PrintString 0 "Need a controller"))))

(event EventOnPhotonCloudInitialized
  (Utilities|FlowControl|Sequence
    (:then_0
      (Utilities|Time|SetTimerbyEvent (delegate Custom|On%20Fake%20Start) 0.2))
    (:then_1
      ;[1 1 1] Connect
      (EventDispatchers|BindEventtoOnPhotonCloudConnected (delegate Custom|On%20Connect))
      (EventDispatchers|BindEventtoOnPlayerJoinedRoom (delegate Custom|On%20Player%20Joined))
      (Class|PhotonCloudObject|SetPlayerName (Guid|ToString(Guid) (Guid|NewGuid)))
      (Class|PhotonCloudObject|Connect))))